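; BP_Turret_Platform is a moving turret that fires Bullet actors at a regular interval.
; The construction script gives InterpToMovement two relative control points, the origin and MovetoPos, with Speed as the travel duration, so higher values move it slower.
; From BeginPlay, a looping Delay spawns a bullet every second at the Arrow component's transform and sets its Force from MyForce.
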(event `self.ReceiveBeginPlay`
  (bind _returnvalue (`|SpawnActorFromClass` "/Game/Sean_H/Blueprints/Bullet.Bullet_C" (`SceneComponent.K2_GetComponentToWorld` (`self.Arrow`)) "Undefined" "MultiplyWithRoot" null null :!label _label))
  (set `/Game/Sean_H/Blueprints/Bullet.Force` (`self.My_Force`) _returnvalue)
  (`KismetSystemLibrary.Delay` 1.0)
  (goto _label))

(fn `UserConstructionScript`
  ;[1 0.0904 0.6951] Moves Turrets Overtime
  (`InterpToMovementComponent.AddControlPointPosition` (`self.InterpToMovement`) (0.0 0.0 0.0) true)
  (`InterpToMovementComponent.AddControlPointPosition` (`self.InterpToMovement`) (`self.MovetoPos`) true)
  (set `InterpToMovementComponent.Duration` (`self.Speed`) (`self.InterpToMovement`)))